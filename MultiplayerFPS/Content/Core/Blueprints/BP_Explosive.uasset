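; BP_Explosive is a thrown grenade-style actor that launches itself with a fixed velocity shortly after BeginPlay.
; Thrown activates ProjectileMovement and starts a random mesh rotation, then after a brief delay plays sound and particles, hides the mesh and sets a lifespan.
; It sphere-traces for Pawns at the blast point, but the loops that would gather unique hit actors and send ExplosiveHitMessage damage are disconnected.
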(event `self.ReceiveBeginPlay`
  (`KismetSystemLibrary.Delay` 1.0)
  (`self.Thrown` (600.0 0.0 0.0)))

(event `Thrown`
  (params (Velocity :type "Vector Structure"))
  (bind _projectilemovement (`self.ProjectileMovement`))
  (bind _returnvalue (`SceneComponent.K2_GetComponentLocation` (`self.ExplosiveMesh`)))
  (bind _returnvalue_2 (`SceneComponent.K2_GetComponentLocation` (`self.ExplosiveMesh`)))
  (`|ExecutionSequence`
    (:`then_0`
      (set `MovementComponent.Velocity` Velocity _projectilemovement)
      (`ActorComponent.Activate` _projectilemovement false)
      (`KismetSystemLibrary.Delay` 0.2)
      (`GameplayStatics.PlaySoundAtLocation` "/Game/Core/Audio/Grenade+4.Grenade+4" _returnvalue_2 (struct) 1.0 1.0 0.0 null null null)
      (`GameplayStatics.SpawnEmitterAtLocation` "/Game/StarterContent/Particles/P_Explosion.P_Explosion" _returnvalue_2)
      (`SceneComponent.SetHiddenInGame` (`self.ExplosiveMesh`) true false)
      (`self.SetLifeSpan` 3.0)
      (bind (_outhits _returnvalue_3) (`KismetSystemLibrary.SphereTraceMultiForObjects` _returnvalue _returnvalue 0.0 (`|MakeArray` "ObjectTypeQuery3" :!type "EObjectTypeQuery Enum")))
      (if _returnvalue_3
        _))
    (:`then_1`
      (`KismetSystemLibrary.MoveComponentTo` (`self.ExplosiveMesh`) (0.0 0.0 0.0) (`KismetMathLibrary.RandomRotator` false)))))

(fn `UserConstructionScript`)